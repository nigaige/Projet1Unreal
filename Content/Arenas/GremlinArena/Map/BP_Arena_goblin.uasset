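; Goblin arena Blueprint that closes in once an actor overlaps it, using two cube components as barriers.
; BeginPlay hides both cubes and disables their collision.
; Any actor overlap, with no filter on the actor, waits briefly, then shows the cubes and enables query and physics collision.
; Nothing in the graph hides the cubes again afterward.
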(event EventBeginPlay
  (Development|SetHiddeninGame (Variables|Default|GetCube) true false)
  (Collision|SetCollisionEnabled (Variables|Default|GetCube) "NoCollision"))

(event Collision|EventActorBeginOverlap
  (params (OtherActor :type Actor%20Object%20Reference))
  (Utilities|FlowControl|Delay 0.2)
  (Development|SetHiddeninGame (Variables|Default|GetCube) false false)
  (Collision|SetCollisionEnabled (Variables|Default|GetCube) "QueryAndPhysics"))

(event EventTick
  (params (DeltaSeconds :type Float%20%28single-precision%29)))

(fn ConstructionScript)