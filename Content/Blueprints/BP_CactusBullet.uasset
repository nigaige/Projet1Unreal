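; BP_CactusBullet is a projectile actor that destroys enemies it touches.
; Each Tick it moves along its Direction at Speed, scaled by delta time, without sweeping.
; When its Box begins overlapping an actor tagged Enemy, it destroys both that actor and itself.
; Other overlaps only print a debug boolean showing whether the actor differs from the player character.
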(event OnComponentBeginOverlap(Box)
  (params (OverlappedComponent :type Primitive%20Component%20Object%20Reference) (OtherActor :type Actor%20Object%20Reference) (OtherComp :type Primitive%20Component%20Object%20Reference) (OtherBodyIndex :type Integer) (bFromSweep :type Boolean) (SweepResult :type Hit%20Result%20Structure%20%28by%20ref%29))
  (if (Actor|ActorHasTag OtherActor "Enemy")
    (Actor|DestroyActor OtherActor)
    (Actor|DestroyActor)
    (else
      (Development|PrintString (Utilities|String|ToString(Boolean) (!= OtherActor (Game|GetPlayerCharacter 0)))))))

(event EventTick
  (params (DeltaSeconds :type Float%20%28single-precision%29))
  ;[1 1 1] Bullet Movement
  (Transformation|SetActorLocation (+ (* DeltaSeconds (Variables|Default|GetSpeed) (Variables|Default|GetDirection)) (Transformation|GetActorLocation)) false false))

(fn ConstructionScript)