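; Game mode Blueprint that tracks the player's last checkpoint and handles respawning at it.
; SetCheckpoint stores the given checkpoint as LastCheckpoint.
; If that checkpoint is valid, Respawn moves the existing player character to its RespawnPoint component's location and zeroes movement velocity, rather than spawning a new pawn.
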(event Custom|Respawn
  (bind _returnvalue (Game|GetPlayerCharacter 0))
  (bind _lastcheckpoint (Variables|Default|GetLastCheckpoint))
  ;[1 1 1] Respawn
  (if (Utilities|IsValid _lastcheckpoint)
    (Transformation|SetActorLocation _returnvalue (Transformation|GetWorldLocation (Variables|/Game/Blueprints/BP_CheckPoint.BP_CheckPoint_C|GetRespawnPoint _lastcheckpoint)) false false)
    (Variables|/Script/Engine.MovementComponent|SetVelocity (Variables|/Script/Engine.Character|GetCharacterMovement _returnvalue) "0, 0, 0")))

(event Custom|Set%20Checkpoint
  (params (Checkpoint :type BP%20Check%20Point%20Object%20Reference))
  (Variables|Default|SetLastCheckpoint Checkpoint))

(fn ConstructionScript)