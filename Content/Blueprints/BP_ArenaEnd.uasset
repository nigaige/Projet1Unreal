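; BP_ArenaEnd is an end-of-arena trigger that finishes the level when the player reaches it.
; When the player pawn overlaps its Cylinder component, it disables player input and shows an EndOfLevel widget.
; After a short delay it re-enables input and opens the level referenced by NextScene.
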(event OnComponentBeginOverlap(Cylinder)
  (params (OverlappedComponent :type Primitive%20Component%20Object%20Reference) (OtherActor :type Actor%20Object%20Reference) (OtherComp :type Primitive%20Component%20Object%20Reference) (OtherBodyIndex :type Integer) (bFromSweep :type Boolean) (SweepResult :type Hit%20Result%20Structure%20%28by%20ref%29))
  (bind _returnvalue (Game|GetPlayerController 0))
  (bind _returnvalue_2 (Game|GetPlayerCharacter 0))
  (if (== OtherActor (Game|Player|GetPlayerPawn 0))
    (Input|DisableInput _returnvalue_2 _returnvalue)
    (bind _returnvalue_3 (UserInterface|CreateWidget "/Game/UI/EndOfLevel.EndOfLevel_C"))
    (UserInterface|Viewport|AddtoViewport _returnvalue_3 0)
    (Utilities|FlowControl|Delay 3.0)
    (Input|EnableInput _returnvalue_2 _returnvalue)
    (Game|OpenLevel(byObjectReference) (Variables|Default|Getnext%20scene))))

(event EventBeginPlay)

(event Collision|EventActorBeginOverlap
  (params (OtherActor :type Actor%20Object%20Reference)))

(event EventTick
  (params (DeltaSeconds :type Float%20%28single-precision%29)))

(fn ConstructionScript)