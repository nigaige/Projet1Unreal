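; BP_RespawnPoint is a checkpoint actor that becomes the active respawn point when the player character overlaps it.
; If it is inactive, it loops over every BP_RespawnPoint in the level, marking only itself active and resetting all sphere materials to gray.
; It then turns its own sphere blue and prints a checkpoint message; the respawn itself is not handled here.
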(event Collision|EventActorBeginOverlap
  (params (OtherActor :type Actor%20Object%20Reference))
  (if (== OtherActor (Game|GetPlayerCharacter 0))
    (if (not (Variables|Default|GetisActive))
      (bind _outactors (Actor|GetAllActorsOfClass "BP_RespawnPoint_C"))
      (for _array_element _outactors
        (Variables|BP_RespawnPoint_C|SetisActive _array_element (== _array_element self))
        (Rendering|Material|SetMaterial (Variables|BP_RespawnPoint_C|GetSphere _array_element) 0 "/Game/LevelPrototyping/Materials/MI_PrototypeGrid_Gray.MI_PrototypeGrid_Gray"))
      (Rendering|Material|SetMaterial (Variables|Default|GetSphere) 0 "/Game/LevelPrototyping/Materials/MI_Solid_Blue.MI_Solid_Blue")
      (Development|PrintString "Checkpoint !"))))

(fn ConstructionScript)