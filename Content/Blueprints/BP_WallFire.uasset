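; BP_WallFire is a hazard that drains HP through BP_GameMode while its Box is occupied.
; Box overlaps set a PlayerIn flag for any actor and cache whether the entering actor is BP_Player_Mage.
; A self-calling event loop started on BeginPlay checks these flags after each short delay and applies Damage, skipping it when the cached mage is shielding.
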(event OnComponentBeginOverlap(Box)
  (params (OverlappedComponent :type Primitive%20Component%20Object%20Reference) (OtherActor :type Actor%20Object%20Reference) (OtherComp :type Primitive%20Component%20Object%20Reference) (OtherBodyIndex :type Integer) (bFromSweep :type Boolean) (SweepResult :type Hit%20Result%20Structure%20%28by%20ref%29))
  (Variables|Default|Setplayer%20in true)
  (bind _asbp_player_mage (Utilities|Casting|CastToBP_Player_Mage OtherActor)
    (:then
      (Variables|Default|Setmage _asbp_player_mage)
      (Variables|Default|Setis%20mage true))
    (:CastFailed
      (Variables|Default|Setis%20mage false))))

(event OnComponentEndOverlap(Box)
  (params (OverlappedComponent :type Primitive%20Component%20Object%20Reference) (OtherActor :type Actor%20Object%20Reference) (OtherComp :type Primitive%20Component%20Object%20Reference) (OtherBodyIndex :type Integer))
  (Variables|Default|Setplayer%20in false))

(event Custom|boucle
  (Utilities|FlowControl|Delay 0.3)
  (if (Variables|Default|Getplayer%20in)
    (if (Variables|Default|Getis%20mage)
      (if (Variables|/Game/Blueprints/Character/BP_Player_Mage.BP_Player_Mage_C|GetisShielding (Variables|Default|Getmage))
        (CallFunction|Boucle)
        (else
          (Default|LoseHP (stale EventBeginPlay _asbp_game_mode) (Variables|Default|Getdamage) :!label _label)
          (CallFunction|Boucle)))
      (else
        (goto _label)))
    (else
      (CallFunction|Boucle))))

(event EventBeginPlay
  (bind _asbp_game_mode (Utilities|Casting|CastToBP_GameMode (Game|GetGameMode)))
  (Utilities|FlowControl|Delay 0.3)
  (if (Variables|Default|Getplayer%20in)
    (if (Variables|Default|Getis%20mage)
      (if (Variables|/Game/Blueprints/Character/BP_Player_Mage.BP_Player_Mage_C|GetisShielding (Variables|Default|Getmage))
        (CallFunction|Boucle)
        (else
          (Default|LoseHP _asbp_game_mode (Variables|Default|Getdamage) :!label _label)
          (CallFunction|Boucle)))
      (else
        (goto _label)))
    (else
      (CallFunction|Boucle))))

(event Collision|EventActorBeginOverlap
  (params (OtherActor :type Actor%20Object%20Reference)))

(event EventTick
  (params (DeltaSeconds :type Float%20%28single-precision%29)))

(event Collision|EventActorEndOverlap
  (params (OtherActor :type Actor%20Object%20Reference)))

(fn ConstructionScript)