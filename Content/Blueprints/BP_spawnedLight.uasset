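; Short-lived point light actor that shrinks away and removes itself after it appears.
; BeginPlay stores the PointLight's attenuation radius in LightForce as the starting value.
; Each Tick reduces LightForce at a fixed, frame-rate-independent rate, clamps it and applies it as the attenuation radius.
; The actor destroys itself when the clamped countdown reaches zero.
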(event EventBeginPlay
  (Variables|Default|Setlight%20force (Variables|/Script/Engine.LocalLightComponent|GetAttenuationRadius (Variables|Default|GetPointLight))))

(event Collision|EventActorBeginOverlap
  (params (OtherActor :type Actor%20Object%20Reference)))

(event EventTick
  (params (DeltaSeconds :type Float%20%28single-precision%29))
  (Rendering|Lighting|SetAttenuationRadius (Variables|Default|GetPointLight) (Math|Float|Clamp(Float) (- (Variables|Default|Getlight%20force) (* DeltaSeconds 4e+02)) 0.0 1e+05))
  (Variables|Default|Setlight%20force (Math|Float|Clamp(Float) (- (Variables|Default|Getlight%20force) (* DeltaSeconds 4e+02)) 0.0 1e+05))
  (if (== (Math|Float|Clamp(Float) (- (Variables|Default|Getlight%20force) (* DeltaSeconds 4e+02)) 0.0 1e+05) 0.0)
    (Actor|DestroyActor)))

(fn ConstructionScript)