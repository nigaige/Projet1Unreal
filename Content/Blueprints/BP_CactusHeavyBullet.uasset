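; BP_CactusHeavyBullet is a projectile that explodes when its Sphere hits any actor other than the player pawn.
; On impact it freezes the Sphere by switching its mobility to Stationary, then plays a timeline that animates the Niagara component's world scale as the explosion.
; When the timeline finishes, it destroys the hit actor if tagged Breakable, then destroys itself.
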(event OnComponentHit(Sphere)
  (params (HitComponent :type Primitive%20Component%20Object%20Reference) (OtherActor :type Actor%20Object%20Reference) (OtherComp :type Primitive%20Component%20Object%20Reference) (NormalImpulse :type Vector :default "0, 0, 0") (Hit :type Hit%20Result%20Structure%20%28by%20ref%29))
  (if (!= OtherActor (Game|Player|GetPlayerPawn 0))
    (Transformation|SetMobility (Variables|Default|GetSphere) "Stationary")
    (bind _explosion_scale (Timeline|Exlpode Play)
      (:Update
        (Transformation|SetWorldScale3D (Variables|Default|GetNiagara) _explosion_scale))
      (:Finished
        (if (Actor|ActorHasTag OtherActor "Breakable")
          (Actor|DestroyActor OtherActor))
        (Actor|DestroyActor)))))

(fn ConstructionScript)