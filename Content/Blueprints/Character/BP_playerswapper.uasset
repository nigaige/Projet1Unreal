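; Player swapper Blueprint that switches control between the Cactus, Mage and Gremlin characters on key presses.
; When the Manager allows a swap, it saves the current pawn's location, rotation and control rotation there, then calls that character's control function.
; Separate events park the parent player far below the world as storage and restart an ice explosion effect when swapped to.
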(event Custom|toStorage
  (Transformation|SetActorLocation (Variables|Default|GetparentPlayer) "0, 0,-10000.000000" false false))

(event Custom|save%20pos
  (bind _returnvalue (Game|Player|GetPlayerPawn 0))
  (bind _manager (Variables|Default|Getmanager))
  (Variables|/Game/Blueprints/Character/manager.manager_C|Setplayer_pos _manager (Transformation|GetActorLocation _returnvalue))
  (Variables|/Game/Blueprints/Character/manager.manager_C|Setplayer_rot _manager (Transformation|GetActorRotation _returnvalue))
  (Variables|/Game/Blueprints/Character/manager.manager_C|Setcamera%20rot _manager (Pawn|GetControlRotation _returnvalue :!class /Script/Engine.Pawn)))

(event Custom|isSwappedTo
  (bind _p_iceexplosion (Variables|Default|GetP_IceExplosion))
  (Components|Activation|Deactivate _p_iceexplosion)
  (Utilities|FlowControl|Delay 0.05)
  (Components|Activation|Activate _p_iceexplosion true))

(event EventBeginPlay
  (bind _returnvalue (Actor|GetActorOfClass "/Game/Blueprints/Character/manager.manager_C"))
  (Variables|Default|Setmanager _returnvalue))

(event Input|KeyboardEvents|Ampersand
  (params (Key :type Key%20Structure :default "None"))
  (:Pressed
    (if (Variables|/Game/Blueprints/Character/manager.manager_C|GetcanSwapChar (Variables|Default|Getmanager))
      (CallFunction|SavePos)
      (Default|ControlCactus (Variables|Default|Getmanager)))))

(event Input|KeyboardEvents|EAccentAigu
  (params (Key :type Key%20Structure :default "None"))
  (:Pressed
    (if (Variables|/Game/Blueprints/Character/manager.manager_C|GetcanSwapChar (Variables|Default|Getmanager))
      (CallFunction|SavePos)
      (Default|ControlMage (Variables|Default|Getmanager)))))

(event Input|KeyboardEvents|Quote
  (params (Key :type Key%20Structure :default "None"))
  (:Pressed
    (if (Variables|/Game/Blueprints/Character/manager.manager_C|GetcanSwapChar (Variables|Default|Getmanager))
      (CallFunction|SavePos)
      (Default|ControlGremlin (Variables|Default|Getmanager)))))

(fn ConstructionScript)