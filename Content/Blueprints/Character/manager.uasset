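; Player character manager that spawns the Cactus, Mage and Gremlin pawns and switches control between them.
; BeginPlay spawns all three, stores them and activates the one chosen by StarterChar.
; Control events call a shared change-player graph unless that pawn is already possessed.
; Each swap stores every body via its PlayerSwaper, possesses the new pawn, applies shared position and rotation, restores camera rotation after a brief delay and updates the GameMode's current player.
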(event Custom|control%20cactus
  (bind _cactus (Variables|Default|Getcactus))
  (if (!= _cactus (Game|Player|GetPlayerPawn 0))
    (Utilities|ChangePlayer _cactus (Variables|/Game/Blueprints/Character/BP_Player_Cactus.BP_Player_Cactus_C|GetPlayerSwaper (stale EventBeginPlay _output_get)))))

(event Custom|control%20mage
  (bind _mage (Variables|Default|GetMage))
  (if (!= _mage (Game|Player|GetPlayerPawn 0))
    (Utilities|ChangePlayer _mage (Variables|/Game/Blueprints/Character/BP_Player_Mage.BP_Player_Mage_C|GetPlayerSwaper (stale EventBeginPlay _output_get_2)))))

(event Custom|control%20gremlin
  (bind _gremlin (Variables|Default|Getgremlin))
  (if (!= _gremlin (Game|Player|GetPlayerPawn 0))
    (Utilities|ChangePlayer _gremlin (Variables|/Game/Blueprints/Character/Gremlin/BP_Player_Gremlin.BP_Player_Gremlin_C|GetPlayerSwaper (stale EventBeginPlay _output_get_3)))))

(event Custom|store%20player
  ;[1 1 1] store player body
  (Default|ToStorage (Variables|/Game/Blueprints/Character/BP_Player_Cactus.BP_Player_Cactus_C|GetPlayerSwaper (Variables|Default|Getcactus_ref)))
  (Default|ToStorage (Variables|/Game/Blueprints/Character/BP_Player_Mage.BP_Player_Mage_C|GetPlayerSwaper (Variables|Default|Getmage_ref)))
  (Default|ToStorage (Variables|/Game/Blueprints/Character/Gremlin/BP_Player_Gremlin.BP_Player_Gremlin_C|GetPlayerSwaper (Variables|Default|Getgremlin_ref)))
  (Default|ShieldInactive (Variables|Default|Getgamemode)))

(event EventBeginPlay
  (bind _asbp_game_mode (Utilities|Casting|CastToBP_GameMode (Game|GetGameMode)))
  (Variables|Default|Setgamemode _asbp_game_mode)
  (bind _returnvalue (Game|SpawnActorfromClass "/Game/Blueprints/Character/BP_Player_Cactus.BP_Player_Cactus_C" (Transformation|GetActorTransform) "Undefined" 0 0))
  (Variables|Default|Setcactus _returnvalue)
  (bind _output_get (Variables|Default|Setcactus_ref _returnvalue))
  (bind _returnvalue_2 (Game|SpawnActorfromClass "/Game/Blueprints/Character/BP_Player_Mage.BP_Player_Mage_C" (Transformation|GetActorTransform) "Undefined" 0 0))
  (Variables|Default|SetMage _returnvalue_2)
  (bind _output_get_2 (Variables|Default|Setmage_ref _returnvalue_2))
  (bind _returnvalue_3 (Game|SpawnActorfromClass "/Game/Blueprints/Character/Gremlin/BP_Player_Gremlin.BP_Player_Gremlin_C" (Transformation|GetActorTransform) "Undefined" 0 0))
  (Variables|Default|Setgremlin _returnvalue_3)
  (bind _output_get_3 (Variables|Default|Setgremlin_ref _returnvalue_3))
  (Default|SavePos (Variables|/Game/Blueprints/Character/Gremlin/BP_Player_Gremlin.BP_Player_Gremlin_C|GetPlayerSwaper _output_get_3))
  (CallFunction|StorePlayer)
  (switch int (Variables|Default|GetstarterChar) ; Allow to define which is the char to be used in the scene:\ndefault / 0 => gremlin\n1 => cactus\n2 => mage
    (:0
      (Utilities|ChangePlayer (Variables|Default|Getgremlin) (Variables|/Game/Blueprints/Character/Gremlin/BP_Player_Gremlin.BP_Player_Gremlin_C|GetPlayerSwaper _output_get_3)))
    (:1
      (Utilities|ChangePlayer (Variables|Default|Getcactus) (Variables|/Game/Blueprints/Character/BP_Player_Cactus.BP_Player_Cactus_C|GetPlayerSwaper _output_get)))
    (:2
      (Utilities|ChangePlayer (Variables|Default|GetMage) (Variables|/Game/Blueprints/Character/BP_Player_Mage.BP_Player_Mage_C|GetPlayerSwaper _output_get_2)))))

(event Collision|EventActorBeginOverlap
  (params (OtherActor :type Actor%20Object%20Reference)))

(fn ConstructionScript)