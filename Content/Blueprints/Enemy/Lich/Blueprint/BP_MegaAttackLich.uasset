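; BP_MegaAttackLich is the Lich enemy's mega attack hazard, which damages the player over time while they overlap it.
; When an actor tagged Player begins overlapping, it prints a taunt and starts a looping half-second timer, which is cleared when the overlap ends.
; Each tick of the timer removes health through LoseHP on the BP_GameMode reference cached at BeginPlay.
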(event Custom|Take%20Damage
  (Default|LoseHP (Variables|Default|GetGamemode) 1))

(event Custom|Stop%20taking%20damage
  (Utilities|Time|ClearandInvalidateTimerbyHandle (stale Custom|Start%20taking%20damage _returnvalue)))

(event Custom|Start%20taking%20damage
  (bind _returnvalue (Utilities|Time|SetTimerbyEvent (delegate Custom|Take%20Damage) 0.5 true)))

(event EventBeginPlay
  (bind _asbp_game_mode (Utilities|Casting|CastToBP_GameMode (Game|GetGameMode)))
  (Variables|Default|Setgamemode _asbp_game_mode))

(event Collision|EventActorBeginOverlap
  (params (OtherActor :type Actor%20Object%20Reference))
  (if (Actor|ActorHasTag OtherActor "Player")
    (Development|PrintString "BURN IN HELL")
    (CallFunction|StartTakingDamage)))

(event Collision|EventActorEndOverlap
  (params (OtherActor :type Actor%20Object%20Reference))
  (if (Actor|ActorHasTag OtherActor "Player")
    (CallFunction|StopTakingDamage)))

(fn ConstructionScript)