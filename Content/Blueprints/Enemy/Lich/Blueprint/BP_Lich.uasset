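; BP_Lich is a lich boss that alternates shielded fireball phases with vulnerable phases.
; Tick checks shield and HP to advance phases, announcing each change through a ChangePhaseBoss call.
; A looping timer spawns fireballs targeting the player, and damage lowers HP only while the child-actor shield is down.
; Mob-spawning events are empty stubs, and Tick handles nothing past the third phase, leaving later phases unfinished.
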(event Custom|phase%204
  (if (<= (Variables|Default|GetHP) 0.0)
    _))

(event Custom|Start%20phase%204
  (Default|CallChangePhaseBoss)
  (CallFunction|StartSpwaningMobs)
  (Variables|Default|SetHP 15.0))

(event Custom|Phase%203
  (if (not (Variables|Default|GetHas_shield))
    (CallFunction|StartPhase4)
    (Variables|Default|SetState_Phase 4)))

(event Custom|Start%20phase%203
  (Default|CallChangePhaseBoss)
  (CallFunction|ActivateShield)
  (CallFunction|StopSpawningMobs)
  (CallFunction|StartCastingFireBall))

(event Custom|Cast%20Fireball
  ;[1 1 1] cast fire ball
  (Utilities|CastFireBall))

(event Custom|Start%20casting%20Fire%20ball
  ;[1 1 1] cast fire ball
  (bind _returnvalue (Utilities|Time|SetTimerbyEvent (delegate Custom|Cast%20Fireball) 5.0 true)))

(event Custom|Stop%20casting%20fire%20ball
  ;[1 1 1] cast fire ball
  (Utilities|Time|ClearandInvalidateTimerbyHandle (stale Custom|Start%20casting%20Fire%20ball _returnvalue)))

(event Custom|Stop%20spawning%20mobs
  ;[1 1 1] Spawner
)

(event Custom|Start%20spwaning%20mobs
  ;[1 1 1] Spawner
)

(event Custom|Phase%202
  (if (<= (Variables|Default|GetHP) 0.0)
    (CallFunction|StartPhase3)
    (Variables|Default|SetState_Phase 3)))

(event Custom|Phase%205)

(event Custom|Phase%201
  (if (not (Variables|Default|GetHas_shield))
    (CallFunction|StartPhase2)
    (Variables|Default|SetState_Phase 2)))

(event Custom|Deactivate%20Shield
  ;[1 1 1] Shield Lich
  (bind _asbp_shield (Utilities|Casting|CastToBP_Shield (Variables|/Script/Engine.ChildActorComponent|GetChildActor (Variables|Default|GetShield))))
  (Default|DesactivateShield _asbp_shield)
  (Variables|Default|SetHas_shield false))

(event Custom|Activate%20Shield
  ;[1 1 1] Shield Lich
  (bind _asbp_shield (Utilities|Casting|CastToBP_Shield (Variables|/Script/Engine.ChildActorComponent|GetChildActor (Variables|Default|GetShield))))
  (Default|ActivateShield _asbp_shield)
  (Variables|Default|SetHas_shield true))

(event Custom|Start%20Phase%201
  (CallFunction|ActivateShield)
  (CallFunction|StartCastingFireBall))

(event Custom|Start%20phase%202
  (Default|CallChangePhaseBoss)
  (CallFunction|StopCastingFireBall)
  (CallFunction|StartSpwaningMobs)
  (Variables|Default|SetHP 15.0))

(event EventBeginPlay
  (CallFunction|StartPhase1))

(event Collision|EventActorBeginOverlap
  (params (OtherActor :type Actor%20Object%20Reference)))

(event EventTick
  (params (DeltaSeconds :type Float%20%28single-precision%29))
  (switch int (Variables|Default|GetState_Phase)
    (:Default
      (CallFunction|Phase1 :!label _label))
    (:0
      (goto _label))
    (:1
      (goto _label))
    (:2
      (CallFunction|Phase2))
    (:3
      (CallFunction|Phase3))))

(event Game|Damage|EventAnyDamage
  (params (Damage :type Float%20%28single-precision%29) (DamageType :type Damage%20Type%20Object%20Reference) (InstigatedBy :type Controller%20Object%20Reference) (DamageCauser :type Actor%20Object%20Reference))
  (if (not (Variables|Default|GetHas_shield))
    (Development|PrintString (Utilities|String|ToString(Float) (Variables|Default|GetHP)))
    (Variables|Default|SetHP (Math|Float|Clamp(Float) (- (Variables|Default|GetHP) Damage) 0.0 15.0))))

(fn ConstructionScript)