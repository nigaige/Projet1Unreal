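; Fireball projectile for the Lich enemy that damages the player through the game mode and explodes.
; On spawn, a timeline animates its height relative to TargetLocation, then a second moves it toward a point just below that target.
; It explodes when that flight ends or it overlaps anything not tagged Boss, scaling up before destroying itself.
; Player overlaps cost HP even after detonation; Boss overlaps only print a debug string.
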(event OnComponentBeginOverlap(Sphere)
  (params (OverlappedComponent :type Primitive%20Component%20Object%20Reference) (OtherActor :type Actor%20Object%20Reference) (OtherComp :type Primitive%20Component%20Object%20Reference) (OtherBodyIndex :type Integer) (bFromSweep :type Boolean) (SweepResult :type Hit%20Result%20Structure%20%28by%20ref%29))
  (if (Actor|ActorHasTag OtherActor "player")
    (Default|LoseHP (Variables|Default|Getgamemode) 3)
    (if (not (Variables|Default|Gethas%20exploded)) :!label _label
      (CallFunction|Explod)
      (bind _speed (Timeline|Speed Stop)
        (:Update
          (Transformation|SetActorLocation (+ (Transformation|GetActorLocation) (* _speed (Variables|Default|Getdirection))) false false))
        (:Finished
          (CallFunction|Explod))))
    (elif (Actor|ActorHasTag OtherActor "Boss")
      (Development|PrintString "Hello")
      (else
        (goto _label)))))

(event Custom|explod
  ;[1 1 1] explosion
  (Variables|Default|Sethas%20exploded true)
  (bind _scale (Timeline|explosion PlayFromStart)
    (:Update
      (Transformation|SetWorldScale3D (Variables|Default|GetDefaultSceneRoot) (Math|Conversions|ToVector(Float) _scale)))
    (:Finished
      (Actor|DestroyActor))))

(event Custom|shoot
  (Variables|Default|Setdirection (Math|Vector|GetUnitDirection(Vector) (Transformation|GetActorLocation) (+ (Variables|Default|GetTarget%20location) "0,0,-50.000000")))
  (bind _speed (Timeline|Speed PlayFromStart)
    (:Update
      (Transformation|SetActorLocation (+ (Transformation|GetActorLocation) (* _speed (Variables|Default|Getdirection))) false false))
    (:Finished
      (CallFunction|Explod))))

(event EventBeginPlay
  (bind _returnvalue (Transformation|GetActorLocation))
  (bind _target_location (Variables|Default|GetTarget%20location))
  (bind (_x _y) (Math|Vector|BreakVector _returnvalue))
  (bind _z (Math|Vector|BreakVector _target_location))
  (bind _asbp_game_mode (Utilities|Casting|CastToBP_GameMode (Game|GetGameMode)))
  (Variables|Default|Setgamemode _asbp_game_mode)
  (Variables|Default|Setstartpos (Transformation|GetActorLocation))
  (bind _z_pos (Timeline|Z%20axis PlayFromStart)
    (:Update
      (Transformation|SetActorLocation (Math|Vector|MakeVector _x _y (+ (* _z_pos (- (.Z (Math|Vector|BreakVector (Variables|Default|Getstartpos))) _z)) _z)) false false))
    (:Finished
      (CallFunction|Shoot))))

(fn ConstructionScript)