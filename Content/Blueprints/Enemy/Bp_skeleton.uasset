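; Skeleton enemy that turns toward the player, chases them once seen through PawnSensing, and registers in BP_Arena_goblin's enemy count.
; An optional BP_Shield child actor absorbs one push.
; Unshielded pushes briefly switch the capsule to physics for a radial and upward launch, which Tick switches off once vertical motion settles.
; Damage has a short invulnerability timer, and death decrements the arena count before destroying the actor.
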(event OnSeePawn(PawnSensing)
  (params (Pawn :type Pawn%20Object%20Reference))
  ;[1 1 1] Follow_Player
  (Variables|Default|SetIs_seeing_player true)
  (CallFunction|FollowPlayer))

(event Custom|Follow_Player
  ;[1 1 1] Follow_Player
  (if (Variables|Default|GetIs_seeing_player)
    (AI|AIMoveTo self "0, 0, 0" (Game|GetPlayerCharacter 0) 5.0 false)))

(event Custom|Can%20retake%20damage
  ;[1 1 1] Comment
  (Variables|Default|SetCan_take_damage true))

(event Custom|get%20impulsed
  (params (Origin :type Vector))
  ;[1 1 1] Get_impulsed
  (if (Variables|Default|GetHas_Shield_Push)
    (bind _asbp_shield (Utilities|Casting|CastToBP_Shield (Variables|/Script/Engine.ChildActorComponent|GetChildActor (Variables|Default|GetChildActor))))
    (Default|ShieldDestroy _asbp_shield)
    (Variables|Default|SetHas_Shield_Push false)
    (else
      (Physics|SetSimulatePhysics (Variables|Collision|GetCapsuleComponent) true)
      (Physics|AddRadialImpulse (Variables|Collision|GetCapsuleComponent) Origin 4e+03 1e+03 "RIF_Constant" true)
      (Physics|AddImpulse (Variables|Collision|GetCapsuleComponent) "0.000000,50.000000,500.000000" "None" true)
      (Variables|Default|SetIs_impulsed true)
      (Utilities|FlowControl|Delay 0.7)
      (Variables|Default|SetIs_impulsed false))))

(event EventBeginPlay
  (bind _returnvalue (Actor|GetActorOfClass "/Game/Arenas/GremlinArena/Map/BP_Arena_goblin.BP_Arena_goblin_C"))
  (Math|Integer|IncrementInt (Variables|/Game/Arenas/GremlinArena/Map/BP_Arena_goblin.BP_Arena_goblin_C|GetNumber_of_Enemy _returnvalue)
    (:%20%20
      (Variables|Default|SetLife_points 3.0)
      (if (Variables|Default|GetHas_Shield_Push)
        (bind _asbp_shield (Utilities|Casting|CastToBP_Shield (Variables|/Script/Engine.ChildActorComponent|GetChildActor (Variables|Default|GetChildActor))))
        (Default|ActivateShield _asbp_shield)))))

(event Game|Damage|EventAnyDamage
  (params (Damage :type Float%20%28single-precision%29) (DamageType :type Damage%20Type%20Object%20Reference) (InstigatedBy :type Controller%20Object%20Reference) (DamageCauser :type Actor%20Object%20Reference))
  ;[1 1 1] Comment
  (if (Variables|Default|GetCan_take_damage)
    (Utilities|Time|SetTimerbyEvent (delegate Custom|Can%20retake%20damage) 0.5)
    (Variables|Default|SetCan_take_damage false)
    (Variables|Default|SetLife_points (Math|Float|Clamp(Float) (- (Variables|Default|GetLife_points) Damage) 0.0 3.0))
    (Development|PrintString (Utilities|String|ToString(Float) (Variables|Default|GetLife_points)))
    (if (== (Variables|Default|GetLife_points) 0.0)
      (bind _returnvalue (Actor|GetActorOfClass "/Game/Arenas/GremlinArena/Map/BP_Arena_goblin.BP_Arena_goblin_C"))
      (Math|Integer|DecrementInt (Variables|/Game/Arenas/GremlinArena/Map/BP_Arena_goblin.BP_Arena_goblin_C|GetNumber_of_Enemy _returnvalue)
        (:%20%20
          (Actor|DestroyActor))))))

(event EventTick
  (params (DeltaSeconds :type Float%20%28single-precision%29))
  ;[1 1 1] Get_impulsed
  (Utilities|FlowControl|Sequence
    (:then_0
      (Transformation|SetActorRotation (|CollapseGraph_0) true))
    (:then_2
      (if (and (< (Math|Float|Absolute(Float) (.Z (Class|KismetMathLibrary|BreakVector3f (Transformation|GetComponentVelocity (Variables|Collision|GetCapsuleComponent))))) 1.0) (not (Variables|Default|GetIs_impulsed)))
        (Physics|SetSimulatePhysics (Variables|Collision|GetCapsuleComponent) false)))))

(fn ConstructionScript)