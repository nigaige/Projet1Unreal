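; BP_Shield is an enemy shield actor that shows or hides a shield effect component on demand.
; It hides the PShieldv202 component on BeginPlay, and Activateshield and Desactivateshield toggle its visibility along with its activation.
; A separate shield_destroy event destroys the actor, while the overlap and Tick events do nothing.
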(event Custom|shield_destroy
  (Actor|DestroyActor))

(event Custom|Desactivate%20shield
  (Development|SetHiddeninGame (Variables|Default|GetP_Shieldv2_02) true true)
  (Components|Activation|Deactivate (Variables|Default|GetP_Shieldv2_02)))

(event Custom|Activate%20%20shield
  (Development|SetHiddeninGame (Variables|Default|GetP_Shieldv2_02) false true)
  (Components|Activation|Activate (Variables|Default|GetP_Shieldv2_02) false))

(event EventBeginPlay
  (Development|SetHiddeninGame (Variables|Default|GetP_Shieldv2_02) true true))

(event Collision|EventActorBeginOverlap
  (params (OtherActor :type Actor%20Object%20Reference)))

(event EventTick
  (params (DeltaSeconds :type Float%20%28single-precision%29)))

(fn ConstructionScript)